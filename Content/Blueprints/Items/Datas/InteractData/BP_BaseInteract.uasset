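; Base interactable Blueprint: a mesh with a sphere trigger that makes itself known to nearby characters.
; The construction script applies the configurable mesh, scale, material and trigger radius.
; Trigger overlaps register and unregister the actor with BP_Character through interactable messages.
; SetOutline toggles custom depth rendering on the mesh for highlighting.
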(event OnComponentBeginOverlap(TriggerInteract)
  (params (OverlappedComponent :type Primitive%20Component%20Object%20Reference) (OtherActor :type Actor%20Object%20Reference) (OtherComp :type Primitive%20Component%20Object%20Reference) (OtherBodyIndex :type Integer) (bFromSweep :type Boolean) (SweepResult :type Hit%20Result%20Structure%20%28by%20ref%29))
  (bind _asbp_character (Utilities|Casting|CastToBP_Character OtherActor))
  (Class|BPIInteract|RegisterInteractable(Message) _asbp_character self))

(event OnComponentEndOverlap(TriggerInteract)
  (params (OverlappedComponent :type Primitive%20Component%20Object%20Reference) (OtherActor :type Actor%20Object%20Reference) (OtherComp :type Primitive%20Component%20Object%20Reference) (OtherBodyIndex :type Integer))
  (bind _asbp_character (Utilities|Casting|CastToBP_Character OtherActor))
  (Class|BPIInteract|UnregisterInteractable(Message) _asbp_character self))

(fn ConstructionScript
  (bind _sm_item (Variables|Default|GetSM_Item))
  (Transformation|SetWorldScale3D _sm_item (Variables|Mesh|GetMeshScale))
  (Components|StaticMesh|SetStaticMesh _sm_item (Variables|Mesh|GetMesh))
  (Rendering|Material|SetMaterial _sm_item 0 (Variables|Mesh|GetMaterial))
  (Components|Sphere|SetSphereRadius (Variables|Default|GetTriggerInteract) (Variables|Trigger|GetTriggerSize) true))

(fn SetOutline
  (params (Outlight? :type Boolean))
  (Rendering|SetRenderCustomDepth (Variables|Default|GetSM_Item) Outlight?))