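; Door Blueprint that moves vertically in response to an interaction and to a BP_Character walking into its trigger, each path playing a sound at the door.
; Interaction removes its trigger, slides the button item along X, then after a delay chained off the timeline's Update destroys the item and runs the DoorLocationDown timeline.
; Overlapping TriggerDoor destroys that trigger, making it one-shot, and runs the DoorLocationUp timeline on the door mesh.
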(event OnComponentBeginOverlap(TriggerDoor)
  (params (OverlappedComponent :type Primitive%20Component%20Object%20Reference) (OtherActor :type Actor%20Object%20Reference) (OtherComp :type Primitive%20Component%20Object%20Reference) (OtherBodyIndex :type Integer) (bFromSweep :type Boolean) (SweepResult :type Hit%20Result%20Structure%20%28by%20ref%29))
  (bind _sm_door (Variables|Default|GetSM_Door))
  (Utilities|Casting|CastToBP_Character OtherActor)
  (Components|DestroyComponent (Variables|Default|GetTriggerDoor))
  (Audio|PlaySoundatLocation "/Game/Sounds/DoorOpenCue.DoorOpenCue" (Transformation|GetWorldLocation _sm_door) "0, 0, 0" 1.0 1.0 0.0 0 0 0)
  (bind _locationz (Timeline|DoorLocationUp Play)
    (:Update
      (Transformation|SetRelativeLocation _sm_door (Math|Vector|MakeVector 57.0 0.0 _locationz) false false))))

(event EventInteraction
  (params (Character :type BP%20Character%20Object%20Reference))
  (bind _sm_item (Variables|Default|GetSM_Item))
  (bind _sm_door (Variables|Default|GetSM_Door))
  (Components|DestroyComponent (Variables|Default|GetTriggerInteract))
  (bind _locationx (Timeline|ButtonLocation Play)
    (:Update
      (Transformation|SetRelativeLocation _sm_item (Math|Vector|MakeVector _locationx 0.0 0.0) false false)
      (Utilities|FlowControl|Delay 2.0)
      (Components|DestroyComponent _sm_item)
      (Audio|PlaySoundatLocation "/Game/Sounds/DoorOpenCue.DoorOpenCue" (Transformation|GetWorldLocation _sm_door) "0, 0, 0" 1.0 1.0 0.0 0 0 0)
      (bind _locationz (Timeline|DoorLocationDown Play)
        (:Update
          (Transformation|SetRelativeLocation _sm_door (Math|Vector|MakeVector 57.0 0.0 _locationz) false false))))))

(fn ConstructionScript
  (|CallParentFunction))