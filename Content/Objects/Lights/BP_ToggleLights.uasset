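; BP_ToggleLights is a trigger actor that switches BP_CubeLight actors when a BP_Character overlaps it.
; It finds every cube light in the level and affects those matching its Group, with Group 0 matching all.
; The Toggle enum selects turning them on, off or randomly on through each light's own functions.
; An optional Destroy flag removes the trigger component on overlap, making it single-use.
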(event OnComponentBeginOverlap(Trigger)
  (params (OverlappedComponent :type Primitive%20Component%20Object%20Reference) (OtherActor :type Actor%20Object%20Reference) (OtherComp :type Primitive%20Component%20Object%20Reference) (OtherBodyIndex :type Integer) (bFromSweep :type Boolean) (SweepResult :type Hit%20Result%20Structure%20%28by%20ref%29))
  (bind _group (Variables|Config|GetGroup))
  (bind _toggle (Variables|Config|GetToggle))
  (Utilities|Casting|CastToBP_Character OtherActor)
  (if (Variables|Config|GetDestroy)
    (Components|DestroyComponent (Variables|Default|GetTrigger)))
  (bind _outactors (Actor|GetAllActorsOfClass "/Game/Objects/Lights/BP_CubeLight.BP_CubeLight_C"))
  (for _array_element _outactors
    (if (or (== (Variables|/Game/Objects/Lights/BP_CubeLight.BP_CubeLight_C|GetGroup _array_element) _group) (== _group 0))
      (if (Utilities|Enum|Equal(Enum) _toggle "NewEnumerator0")
        (Default|Toggleon _array_element)
        (elif (Utilities|Enum|Equal(Enum) _toggle "NewEnumerator1")
          (Default|ToggleOff _array_element)
          (elif (Utilities|Enum|Equal(Enum) _toggle "NewEnumerator2")
            (Default|ToggleonRandom _array_element)))))))

(fn ConstructionScript)