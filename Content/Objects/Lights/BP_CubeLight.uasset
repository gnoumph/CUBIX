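; BP_CubeLight is a light prop whose cube mesh and child light components switch on, off, or on after a random delay.
; An enum, applied on BeginPlay or through StartLight, selects the mode.
; Each mode sets the intensity of the child lights, scaled by a multiplier, alongside the cube material's Emissive parameter.
; The random mode turns everything off, waits up to two seconds, then drives both from an Intensity timeline.
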(event Custom|StartLight
  (params (Toggle :type S_Toggle%20Enum :default "NewEnumerator0"))
  (Variables|Config|SetToggle Toggle)
  (if (Utilities|Enum|Equal(Enum) (Variables|Config|GetToggle) "NewEnumerator0")
    (CallFunction|Toggleon)
    (elif (Utilities|Enum|Equal(Enum) (Variables|Config|GetToggle) "NewEnumerator1")
      (CallFunction|ToggleOff)
      (elif (Utilities|Enum|Equal(Enum) (Variables|Config|GetToggle) "NewEnumerator2")
        (CallFunction|ToggleonRandom)))))

(event Custom|SwitchOnRandom
  (bind _sm_cube (Variables|Default|GetSM_Cube))
  (CallFunction|ToggleOff)
  (Utilities|FlowControl|Delay (Math|Random|RandomFloatinRange 0.0 2.0))
  (bind _intensity (Timeline|Intensity Play)
    (:Update
      (Utilities|FlowControl|Sequence
        (:then_0
          (for _array_element (Components|GetChildrenComponents _sm_cube false)
            (bind _aslight_component (Utilities|Casting|CastToLightComponent _array_element))
            (Rendering|Components|Light|SetIntensity _aslight_component (* _intensity (Variables|Config|GetIntensityMultiplier)))))
        (:then_1
          (Rendering|Material|SetScalarParameterValueonMaterials _sm_cube "Emissive" (/ _intensity 1e+03)))))))

(event EventBeginPlay
  (bind _toggle (Variables|Config|GetToggle))
  (if (Utilities|Enum|Equal(Enum) _toggle "NewEnumerator0")
    (CallFunction|Toggleon)
    (elif (Utilities|Enum|Equal(Enum) _toggle "NewEnumerator1")
      (CallFunction|ToggleOff)
      (elif (Utilities|Enum|Equal(Enum) _toggle "NewEnumerator2")
        (CallFunction|ToggleonRandom)))))

(fn ConstructionScript)

(fn Toggleon
  (bind _sm_cube (Variables|Default|GetSM_Cube))
  (Utilities|FlowControl|Sequence
    (:then_0
      (for _array_element (Components|GetChildrenComponents _sm_cube false)
        (bind _aslight_component (Utilities|Casting|CastToLightComponent _array_element))
        (Rendering|Components|Light|SetIntensity _aslight_component (* (Variables|Config|GetIntensityMultiplier) 1e+03))))
    (:then_1
      (Rendering|Material|SetScalarParameterValueonMaterials _sm_cube "Emissive" 1.0))))

(fn ToggleOff
  (bind _sm_cube (Variables|Default|GetSM_Cube))
  (Utilities|FlowControl|Sequence
    (:then_0
      (for _array_element (Components|GetChildrenComponents _sm_cube false)
        (bind _aslight_component (Utilities|Casting|CastToLightComponent _array_element))
        (Rendering|Components|Light|SetIntensity _aslight_component 0.0)))
    (:then_1
      (Rendering|Material|SetScalarParameterValueonMaterials _sm_cube "Emissive" 0.0))))

(fn ToggleonRandom
  (CallFunction|SwitchonRandom))