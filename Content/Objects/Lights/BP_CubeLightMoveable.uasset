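; BP_CubeLightMoveable is a moving cube light that rotates its SMCube component during play.
; On BeginPlay it runs the parent logic, picks a random angle offset for each axis, then plays the Rotation timeline.
; Each timeline update adds those offsets to the shared track value and sets the result as the cube's relative roll, pitch and yaw.
; The construction script only calls the parent's.
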(event EventBeginPlay
  (|CallParentFunction)
  (Variables|Default|SetRandomX (Math|Random|RandomFloatinRange -45.0 45.0))
  (Variables|Default|SetRandomY (Math|Random|RandomFloatinRange -45.0 45.0))
  (Variables|Default|SetRandomZ (Math|Random|RandomFloatinRange -45.0 45.0))
  (bind _rotation (Timeline|Rotation Play)
    (:Update
      (Transformation|SetRelativeRotation (Variables|Default|GetSM_Cube) (Math|Rotator|MakeRotator (+ _rotation (Variables|Default|GetRandomX)) (+ _rotation (Variables|Default|GetRandomY)) (+ _rotation (Variables|Default|GetRandomZ))) false false))))

(fn ConstructionScript
  (|CallParentFunction))