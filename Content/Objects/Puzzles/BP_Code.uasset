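; BP_Code is a code-lock puzzle that opens a door when the correct code is entered.
; On BeginPlay it hands itself to the UI_Code widget shown in its widget component.
; CheckCode compares the entered code to the stored one while the door is closed, then turns the widget off and plays a timeline that moves the referenced door's mesh along Z.
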(event Custom|CheckCode
  (params (CurrentCode :type String))
  (if (and (Utilities|Enum|Equal(Enum) CurrentCode (Variables|Config|GetCode)) (Variables|Default|GetDoorClosed))
    (Variables|Default|SetDoorClosed false)
    (bind _asui_code (Utilities|Casting|CastToUI_Code (UserInterface|GetUserWidgetObject (Variables|Default|GetWidget))))
    (Default|TurnOff _asui_code)
    (bind _down (Timeline|Down Play)
      (:Update
        (Transformation|SetRelativeLocation (Variables|/Game/Objects/Doors/BP_SimpleDoor.BP_SimpleDoor_C|GetDoor (Variables|Config|GetDoor)) (Math|Vector|MakeVector 0.0 0.0 _down) false false)))))

(event EventBeginPlay
  (bind _asui_code (Utilities|Casting|CastToUI_Code (UserInterface|GetUserWidgetObject (Variables|Default|GetWidget))))
  (Variables|/Game/UI/UI_Code.UI_Code_C|SetRefBP_Code _asui_code self))

(fn ConstructionScript)