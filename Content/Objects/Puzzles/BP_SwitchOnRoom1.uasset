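; Puzzle-room trigger that plays a scripted light-up and power-drop sequence when BP_Character first overlaps it, then destroys its trigger component.
; Nested Sequence and Delay nodes switch six wall groups to a light material one after another, each with a positional sound.
; All walls then change to MI_WhiteBrillant around a power-drop sound at the player.
; After a longer pause, it calls StartLight on every BP_CubeLightMoveable and plays a lights-on sound.
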(event Collision|EventActorBeginOverlap
  (params (OtherActor :type Actor%20Object%20Reference))
  (bind _wall5 (Variables|Walls|GetWall5))
  (bind _wall2 (Variables|Walls|GetWall2))
  (bind _wall1a (Variables|Walls|GetWall1a))
  (bind _wall1c (Variables|Walls|GetWall1c))
  (bind _wall3 (Variables|Walls|GetWall3))
  (bind _wall4 (Variables|Walls|GetWall4))
  (bind _staticmeshcomponent (Variables|/Script/Engine.StaticMeshActor|GetStaticMeshComponent _wall5))
  (bind _staticmeshcomponent_2 (Variables|/Script/Engine.StaticMeshActor|GetStaticMeshComponent _wall1c))
  (bind _staticmeshcomponent_3 (Variables|/Script/Engine.StaticMeshActor|GetStaticMeshComponent _wall1a))
  (bind _staticmeshcomponent_4 (Variables|/Script/Engine.StaticMeshActor|GetStaticMeshComponent _wall2))
  (bind _staticmeshcomponent_5 (Variables|/Script/Engine.StaticMeshActor|GetStaticMeshComponent _wall3))
  (bind _staticmeshcomponent_6 (Variables|/Script/Engine.StaticMeshActor|GetStaticMeshComponent _wall4))
  (bind _returnvalue (Transformation|GetWorldLocation _staticmeshcomponent_2))
  (Utilities|Casting|CastToBP_Character OtherActor)
  (Utilities|FlowControl|Sequence
    (:then_0
      (Rendering|Material|SetMaterial _staticmeshcomponent_3 0 "/Game/Materials/MI_LightMat.MI_LightMat")
      (Utilities|FlowControl|Delay 2.0)
      (Utilities|FlowControl|Sequence
        (:then_0
          (Rendering|Material|SetMaterial _staticmeshcomponent_4 0 "/Game/Materials/MI_LightMat.MI_LightMat")
          (Utilities|FlowControl|Delay 1.0)
          (Utilities|FlowControl|Sequence
            (:then_0
              (Rendering|Material|SetMaterial _staticmeshcomponent_5 0 "/Game/Materials/MI_LightMat.MI_LightMat")
              (Utilities|FlowControl|Delay 1.0)
              (Utilities|FlowControl|Sequence
                (:then_0
                  (Rendering|Material|SetMaterial _staticmeshcomponent_6 0 "/Game/Materials/MI_LightMat.MI_LightMat")
                  (Utilities|FlowControl|Delay 1.0)
                  (Utilities|FlowControl|Sequence
                    (:then_0
                      (Rendering|Material|SetMaterial _staticmeshcomponent 0 "/Game/Materials/MI_LightMat.MI_LightMat")
                      (Utilities|FlowControl|Delay 1.0)
                      (Utilities|FlowControl|Sequence
                        (:then_0
                          (Rendering|Material|SetMaterial (Variables|/Script/Engine.StaticMeshActor|GetStaticMeshComponent (Variables|Walls|GetWall6a)) 0 "/Game/Materials/MI_LightMat.MI_LightMat")
                          (Utilities|FlowControl|Sequence
                            (:then_0
                              (Utilities|FlowControl|Delay 2.0)
                              (Rendering|Material|SetMaterial _staticmeshcomponent_3 0 "/Game/Materials/MI_WhiteBrillant.MI_WhiteBrillant")
                              (Utilities|FlowControl|Delay 8.0)
                              (Utilities|FlowControl|Sequence
                                (:then_0
                                  (bind _outactors (Actor|GetAllActorsOfClass "/Game/Objects/Lights/BP_CubeLightMoveable.BP_CubeLightMoveable_C"))
                                  (for _array_element _outactors
                                    (Default|StartLight _array_element "NewEnumerator2")))
                                (:then_1
                                  (Audio|PlaySoundatLocation "/Game/Sounds/LightsOnCue.LightsOnCue" _returnvalue "0, 0, 0" 1.0 1.0 0.0 0 0 0))))
                            (:then_1
                              (Utilities|FlowControl|Delay 1.8)
                              (Audio|PlaySoundatLocation "/Game/Sounds/PowerDropCue.PowerDropCue" (Transformation|GetWorldLocation (Variables|/Script/Engine.Character|GetMesh (Game|GetPlayerCharacter 0))) "0, 0, 0" 1.0 1.0 0.0 0 0 0))))
                        (:then_1
                          (Audio|PlaySoundatLocation "/Game/Sounds/BigLightOn2Cue.BigLightOn2Cue" (Transformation|GetWorldLocation (Variables|/Script/Engine.StaticMeshActor|GetStaticMeshComponent (Variables|Walls|GetWall6c))) "0, 0, 0" 1.0 1.0 0.0 0 0 0))))
                    (:then_1
                      (Audio|PlaySoundatLocation "/Game/Sounds/BigLightOn1Cue.BigLightOn1Cue" (Transformation|GetWorldLocation _staticmeshcomponent) "0, 0, 0" 1.0 1.0 0.0 0 0 0))))
                (:then_1
                  (Audio|PlaySoundatLocation "/Game/Sounds/BigLightOn1Cue.BigLightOn1Cue" (Transformation|GetWorldLocation _staticmeshcomponent_6) "0, 0, 0" 1.0 1.0 0.0 0 0 0))))
            (:then_1
              (Audio|PlaySoundatLocation "/Game/Sounds/BigLightOn1Cue.BigLightOn1Cue" (Transformation|GetWorldLocation _staticmeshcomponent_5) "0, 0, 0" 1.0 1.0 0.0 0 0 0))))
        (:then_1
          (Audio|PlaySoundatLocation "/Game/Sounds/BigLightOn1Cue.BigLightOn1Cue" (Transformation|GetWorldLocation _staticmeshcomponent_4) "0, 0, 0" 1.0 1.0 0.0 0 0 0))))
    (:then_1
      (Components|DestroyComponent (Variables|Default|GetTrigger)))
    (:then_2
      (Audio|PlaySoundatLocation "/Game/Sounds/BigLightOn1Cue.BigLightOn1Cue" _returnvalue "0, 0, 0" 1.0 1.0 0.0 0 0 0))))

(fn ConstructionScript)