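; Sequence puzzle in which four pressure plates must be stepped on in order to open a series of door bars.
; Overlap triggers placed above each plate animate it down and back via timelines and update progress flags in SetDoors.
; Plate 1 restarts the sequence, while any other out-of-order step resets it.
; MoveBar plays or reverses bar timelines from those flags, with the final step sliding three bars sideways.
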(event OnComponentBeginOverlap(Trigger1)
  (params (OverlappedComponent :type Primitive%20Component%20Object%20Reference) (OtherActor :type Actor%20Object%20Reference) (OtherComp :type Primitive%20Component%20Object%20Reference) (OtherBodyIndex :type Integer) (bFromSweep :type Boolean) (SweepResult :type Hit%20Result%20Structure%20%28by%20ref%29))
  (bind _initialposition1 (Variables|Positions|GetInitialPosition1))
  ;[1 1 1] Trigger zones
  (CallFunction|SetDoors OverlappedComponent)
  (bind _down (Timeline|Down1 Play)
    (:Update
      (Transformation|SetRelativeLocation (Variables|/Script/Engine.StaticMeshActor|GetStaticMeshComponent (Variables|Zones|GetZone1)) (Math|Vector|MakeVector (.x _initialposition1) (.y _initialposition1) (- (.z _initialposition1) _down)) false false))))

(event OnComponentEndOverlap(Trigger1)
  (params (OverlappedComponent :type Primitive%20Component%20Object%20Reference) (OtherActor :type Actor%20Object%20Reference) (OtherComp :type Primitive%20Component%20Object%20Reference) (OtherBodyIndex :type Integer))
  (bind _initialposition1 (Variables|Positions|GetInitialPosition1))
  ;[1 1 1] Trigger zones
  (bind _down (Timeline|Down1 Reverse)
    (:Update
      (Transformation|SetRelativeLocation (Variables|/Script/Engine.StaticMeshActor|GetStaticMeshComponent (Variables|Zones|GetZone1)) (Math|Vector|MakeVector (.x _initialposition1) (.y _initialposition1) (- (.z _initialposition1) _down)) false false))))

(event OnComponentBeginOverlap(Trigger2)
  (params (OverlappedComponent :type Primitive%20Component%20Object%20Reference) (OtherActor :type Actor%20Object%20Reference) (OtherComp :type Primitive%20Component%20Object%20Reference) (OtherBodyIndex :type Integer) (bFromSweep :type Boolean) (SweepResult :type Hit%20Result%20Structure%20%28by%20ref%29))
  (bind _initialposition2 (Variables|Positions|GetInitialPosition2))
  ;[1 1 1] Trigger zones
  (CallFunction|SetDoors OverlappedComponent)
  (bind _down (Timeline|Down2 Play)
    (:Update
      (Transformation|SetRelativeLocation (Variables|/Script/Engine.StaticMeshActor|GetStaticMeshComponent (Variables|Zones|GetZone2)) (Math|Vector|MakeVector (.x _initialposition2) (.y _initialposition2) (- (.z _initialposition2) _down)) false false))))

(event OnComponentEndOverlap(Trigger2)
  (params (OverlappedComponent :type Primitive%20Component%20Object%20Reference) (OtherActor :type Actor%20Object%20Reference) (OtherComp :type Primitive%20Component%20Object%20Reference) (OtherBodyIndex :type Integer))
  (bind _initialposition2 (Variables|Positions|GetInitialPosition2))
  ;[1 1 1] Trigger zones
  (bind _down (Timeline|Down2 Reverse)
    (:Update
      (Transformation|SetRelativeLocation (Variables|/Script/Engine.StaticMeshActor|GetStaticMeshComponent (Variables|Zones|GetZone2)) (Math|Vector|MakeVector (.x _initialposition2) (.y _initialposition2) (- (.z _initialposition2) _down)) false false))))

(event OnComponentBeginOverlap(Trigger3)
  (params (OverlappedComponent :type Primitive%20Component%20Object%20Reference) (OtherActor :type Actor%20Object%20Reference) (OtherComp :type Primitive%20Component%20Object%20Reference) (OtherBodyIndex :type Integer) (bFromSweep :type Boolean) (SweepResult :type Hit%20Result%20Structure%20%28by%20ref%29))
  (bind _initialposition3 (Variables|Positions|GetInitialPosition3))
  ;[1 1 1] Trigger zones
  (CallFunction|SetDoors OverlappedComponent)
  (bind _down (Timeline|Down3 Play)
    (:Update
      (Transformation|SetRelativeLocation (Variables|/Script/Engine.StaticMeshActor|GetStaticMeshComponent (Variables|Zones|GetZone3)) (Math|Vector|MakeVector (.x _initialposition3) (.y _initialposition3) (- (.z _initialposition3) _down)) false false))))

(event OnComponentEndOverlap(Trigger3)
  (params (OverlappedComponent :type Primitive%20Component%20Object%20Reference) (OtherActor :type Actor%20Object%20Reference) (OtherComp :type Primitive%20Component%20Object%20Reference) (OtherBodyIndex :type Integer))
  (bind _initialposition3 (Variables|Positions|GetInitialPosition3))
  ;[1 1 1] Trigger zones
  (bind _down (Timeline|Down3 Reverse)
    (:Update
      (Transformation|SetRelativeLocation (Variables|/Script/Engine.StaticMeshActor|GetStaticMeshComponent (Variables|Zones|GetZone3)) (Math|Vector|MakeVector (.x _initialposition3) (.y _initialposition3) (- (.z _initialposition3) _down)) false false))))

(event OnComponentBeginOverlap(Trigger4)
  (params (OverlappedComponent :type Primitive%20Component%20Object%20Reference) (OtherActor :type Actor%20Object%20Reference) (OtherComp :type Primitive%20Component%20Object%20Reference) (OtherBodyIndex :type Integer) (bFromSweep :type Boolean) (SweepResult :type Hit%20Result%20Structure%20%28by%20ref%29))
  (bind _initialposition4 (Variables|Positions|GetInitialPosition4))
  ;[1 1 1] Trigger zones
  (CallFunction|SetDoors OverlappedComponent)
  (bind _down (Timeline|Down4 Play)
    (:Update
      (Transformation|SetRelativeLocation (Variables|/Script/Engine.StaticMeshActor|GetStaticMeshComponent (Variables|Zones|GetZone4)) (Math|Vector|MakeVector (.x _initialposition4) (.y _initialposition4) (- (.z _initialposition4) _down)) false false))))

(event OnComponentEndOverlap(Trigger4)
  (params (OverlappedComponent :type Primitive%20Component%20Object%20Reference) (OtherActor :type Actor%20Object%20Reference) (OtherComp :type Primitive%20Component%20Object%20Reference) (OtherBodyIndex :type Integer))
  (bind _initialposition4 (Variables|Positions|GetInitialPosition4))
  ;[1 1 1] Trigger zones
  (bind _down (Timeline|Down4 Reverse)
    (:Update
      (Transformation|SetRelativeLocation (Variables|/Script/Engine.StaticMeshActor|GetStaticMeshComponent (Variables|Zones|GetZone4)) (Math|Vector|MakeVector (.x _initialposition4) (.y _initialposition4) (- (.z _initialposition4) _down)) false false))))

(event Custom|MoveBar
  (bind _initialpositiondoor6 (Variables|Positions|GetInitialPositionDoor6))
  (bind _initialpositiondoor1 (Variables|Positions|GetInitialPositionDoor1))
  (bind _initialpositiondoor2 (Variables|Positions|GetInitialPositionDoor2))
  (bind _initialpositiondoor3 (Variables|Positions|GetInitialPositionDoor3))
  (bind _initialpositiondoor4 (Variables|Positions|GetInitialPositionDoor4))
  (bind _initialpositiondoor5 (Variables|Positions|GetInitialPositionDoor5))
  ;[1 1 1] Open doors
  (if (Variables|Doors|GetFirstDoorOpen)
    (Utilities|FlowControl|Sequence
      (:then_0
        (bind _door1z (Timeline|Door1 Play)
          (:Update
            (Transformation|SetRelativeLocation (Variables|/Script/Engine.StaticMeshActor|GetStaticMeshComponent (Variables|Bars|GetBar1)) (Math|Vector|MakeVector (.x _initialpositiondoor1) (.y _initialpositiondoor1) (+ _door1z (.z _initialpositiondoor1))) false false))))
      (:then_1
        (if (and (Variables|Doors|GetFirstDoorOpen) (Variables|Doors|GetSecondDoorOpen)) :!label _label
          (Utilities|FlowControl|Sequence
            (:then_0
              (bind _door2z (Timeline|Door2 Play)
                (:Update
                  (Transformation|SetRelativeLocation (Variables|/Script/Engine.StaticMeshActor|GetStaticMeshComponent (Variables|Bars|GetBar2)) (Math|Vector|MakeVector (.x _initialpositiondoor2) (.y _initialpositiondoor2) (+ _door2z (.z _initialpositiondoor2))) false false))))
            (:then_1
              (if (Math|Boolean|ANDBoolean (Variables|Doors|GetFirstDoorOpen) (Variables|Doors|GetSecondDoorOpen) (Variables|Doors|GetThirdDoorOpen)) :!label _label_2
                (Utilities|FlowControl|Sequence
                  (:then_0
                    (bind _door3z (Timeline|Door3 Play)
                      (:Update
                        (Transformation|SetRelativeLocation (Variables|/Script/Engine.StaticMeshActor|GetStaticMeshComponent (Variables|Bars|GetBar3)) (Math|Vector|MakeVector (.x _initialpositiondoor3) (.y _initialpositiondoor3) (+ _door3z (.z _initialpositiondoor3))) false false))))
                  (:then_1
                    (if (Math|Boolean|ANDBoolean (Variables|Doors|GetFirstDoorOpen) (Variables|Doors|GetSecondDoorOpen) (Variables|Doors|GetThirdDoorOpen) (Variables|Doors|GetFourthDoorOpen)) :!label _label_3
                      (Utilities|FlowControl|Sequence
                        (:then_0
                          (bind _door4y (Timeline|Door4 Play)
                            (:Update
                              (Transformation|SetRelativeLocation (Variables|/Script/Engine.StaticMeshActor|GetStaticMeshComponent (Variables|Bars|GetBar4)) (Math|Vector|MakeVector (.x _initialpositiondoor4) (+ _door4y (.y _initialpositiondoor4)) (.z _initialpositiondoor4)) false false))))
                        (:then_1
                          (bind _door5y (Timeline|Door5 Play)
                            (:Update
                              (Transformation|SetRelativeLocation (Variables|/Script/Engine.StaticMeshActor|GetStaticMeshComponent (Variables|Bars|GetBar5)) (Math|Vector|MakeVector (.x _initialpositiondoor5) (- (.y _initialpositiondoor5) _door5y) (.z _initialpositiondoor5)) false false))))
                        (:then_2
                          (bind _door6y (Timeline|Door6 Play)
                            (:Update
                              (Transformation|SetRelativeLocation (Variables|/Script/Engine.StaticMeshActor|GetStaticMeshComponent (Variables|Bars|GetBar6)) (Math|Vector|MakeVector (.x _initialpositiondoor6) (+ _door6y (.y _initialpositiondoor6)) (.z _initialpositiondoor6)) false false)))))
                      (else
                        (Utilities|FlowControl|Sequence
                          (:then_0
                            (Timeline|Door4 Reverse))
                          (:then_1
                            (Timeline|Door5 Reverse))
                          (:then_2
                            (Timeline|Door6 Reverse)))))))
                (else
                  (Utilities|FlowControl|Sequence
                    (:then_0
                      (Timeline|Door3 Reverse))
                    (:then_1
                      (goto _label_3)))))))
          (else
            (Utilities|FlowControl|Sequence
              (:then_0
                (Timeline|Door2 Reverse))
              (:then_1
                (goto _label_2)))))))
    (else
      (Utilities|FlowControl|Sequence
        (:then_0
          (Timeline|Door1 Reverse))
        (:then_1
          (goto _label))))))

(event EventBeginPlay
  ;[1 1 1] Init positions
  (bind _output_get (Variables|Positions|SetInitialPosition1 (Transformation|GetWorldLocation (Variables|/Script/Engine.StaticMeshActor|GetStaticMeshComponent (Variables|Zones|GetZone1)))))
  (bind _output_get_2 (Variables|Positions|SetInitialPosition2 (Transformation|GetWorldLocation (Variables|/Script/Engine.StaticMeshActor|GetStaticMeshComponent (Variables|Zones|GetZone2)))))
  (bind _output_get_3 (Variables|Positions|SetInitialPosition3 (Transformation|GetWorldLocation (Variables|/Script/Engine.StaticMeshActor|GetStaticMeshComponent (Variables|Zones|GetZone3)))))
  (bind _output_get_4 (Variables|Positions|SetInitialPosition4 (Transformation|GetWorldLocation (Variables|/Script/Engine.StaticMeshActor|GetStaticMeshComponent (Variables|Zones|GetZone4)))))
  (Transformation|SetWorldLocation (Variables|Default|GetTrigger1) (+ _output_get "0, 0,50.000000") false false)
  (Transformation|SetWorldLocation (Variables|Default|GetTrigger2) (+ _output_get_2 "0, 0,50.000000") false false)
  (Transformation|SetWorldLocation (Variables|Default|GetTrigger3) (+ _output_get_3 "0, 0,50.000000") false false)
  (Transformation|SetWorldLocation (Variables|Default|GetTrigger4) (+ _output_get_4 "0, 0,50.000000") false false)
  (Variables|Positions|SetInitialPositionDoor1 (Transformation|GetWorldLocation (Variables|/Script/Engine.StaticMeshActor|GetStaticMeshComponent (Variables|Bars|GetBar1))))
  (Variables|Positions|SetInitialPositionDoor2 (Transformation|GetWorldLocation (Variables|/Script/Engine.StaticMeshActor|GetStaticMeshComponent (Variables|Bars|GetBar2))))
  (Variables|Positions|SetInitialPositionDoor3 (Transformation|GetWorldLocation (Variables|/Script/Engine.StaticMeshActor|GetStaticMeshComponent (Variables|Bars|GetBar3))))
  (Variables|Positions|SetInitialPositionDoor4 (Transformation|GetWorldLocation (Variables|/Script/Engine.StaticMeshActor|GetStaticMeshComponent (Variables|Bars|GetBar4))))
  (Variables|Positions|SetInitialPositionDoor5 (Transformation|GetWorldLocation (Variables|/Script/Engine.StaticMeshActor|GetStaticMeshComponent (Variables|Bars|GetBar5))))
  (Variables|Positions|SetInitialPositionDoor6 (Transformation|GetWorldLocation (Variables|/Script/Engine.StaticMeshActor|GetStaticMeshComponent (Variables|Bars|GetBar6)))))

(fn ConstructionScript)

(fn SetDoors
  (params (Trigger :type Primitive%20Component%20Object%20Reference))
  (if (== Trigger (Variables|Default|GetTrigger1))
    (Variables|Doors|SetFirstDoorOpen true)
    (Variables|Doors|SetSecondDoorOpen false)
    (Variables|Doors|SetThirdDoorOpen false)
    (Variables|Doors|SetFourthDoorOpen false)
    (CallFunction|OpenDoors)
    (elif (== Trigger (Variables|Default|GetTrigger2))
      (if (Math|Boolean|ANDBoolean (Variables|Doors|GetFirstDoorOpen) (not (Variables|Doors|GetSecondDoorOpen)) (not (Variables|Doors|GetThirdDoorOpen)) (not (Variables|Doors|GetFourthDoorOpen)))
        (Variables|Doors|SetSecondDoorOpen true)
        (Variables|Doors|SetThirdDoorOpen false)
        (Variables|Doors|SetFourthDoorOpen false)
        (CallFunction|OpenDoors)
        (else
          (CallFunction|ResetDoors)))
      (elif (== Trigger (Variables|Default|GetTrigger3))
        (if (Math|Boolean|ANDBoolean (Variables|Doors|GetFirstDoorOpen) (Variables|Doors|GetSecondDoorOpen) (not (Variables|Doors|GetThirdDoorOpen)) (not (Variables|Doors|GetFourthDoorOpen)))
          (Variables|Doors|SetThirdDoorOpen true)
          (Variables|Doors|SetFourthDoorOpen false)
          (CallFunction|OpenDoors)
          (else
            (CallFunction|ResetDoors)))
        (elif (== Trigger (Variables|Default|GetTrigger4))
          (if (Math|Boolean|ANDBoolean (Variables|Doors|GetFirstDoorOpen) (Variables|Doors|GetSecondDoorOpen) (Variables|Doors|GetThirdDoorOpen) (not (Variables|Doors|GetFourthDoorOpen)))
            (Variables|Doors|SetFourthDoorOpen true)
            (CallFunction|OpenDoors)
            (else
              (CallFunction|ResetDoors)))
          (else
            (CallFunction|ResetDoors)))))))

(fn OpenDoors
  (CallFunction|MoveBar))

(fn ResetDoors
  (Variables|Doors|SetFirstDoorOpen false)
  (Variables|Doors|SetSecondDoorOpen false)
  (Variables|Doors|SetThirdDoorOpen false)
  (Variables|Doors|SetFourthDoorOpen false)
  (CallFunction|OpenDoors))