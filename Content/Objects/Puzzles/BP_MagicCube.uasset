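; Puzzle cube that changes appearance and switches its linked cube lights whenever the player's physics handle is active.
; Tick polls the player character, using IsTransparent to act only on state changes.
; Activation applies a transparent red material, toggles off same-Group BP_CubeLight actors and plays the Switch timeline driving its light intensity.
; Release restores the brilliant red material, calls ToggleOnRandom on those lights and reverses the timeline.
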(event EventTick
  (params (DeltaSeconds :type Float%20%28single-precision%29))
  (bind _sm_item (Variables|Default|GetSM_Item))
  (|CallParentFunction 0.0)
  (bind _asbp_character (Utilities|Casting|CastToBP_Character (Game|GetPlayerCharacter 0)))
  (if (Variables|/Game/Blueprints/Datas/Character/BP_Character.BP_Character_C|GetPhysicsHandleActive _asbp_character)
    (if (not (Variables|Default|GetIsTransparent?))
      (Rendering|Material|SetMaterial _sm_item 0 "/Game/Materials/MI_RedTransparent.MI_RedTransparent")
      (Variables|Default|SetIsTransparent? true)
      (bind _outactors (Actor|GetAllActorsOfClass "/Game/Objects/Lights/BP_CubeLight.BP_CubeLight_C"))
      (for _array_element _outactors
        (if (== (Variables|/Game/Objects/Lights/BP_CubeLight.BP_CubeLight_C|GetGroup _array_element) (Variables|Default|GetGroup))
          (Default|ToggleOff _array_element)))
      (bind _intensity (Timeline|Switch Play)
        (:Update
          (Rendering|Components|Light|SetIntensity (Variables|Default|GetLight) _intensity))))
    (elif (Variables|Default|GetIsTransparent?)
      (Rendering|Material|SetMaterial _sm_item 0 "/Game/Materials/MI_RedBrillant.MI_RedBrillant")
      (Variables|Default|SetIsTransparent? false)
      (bind _outactors_2 (Actor|GetAllActorsOfClass "/Game/Objects/Lights/BP_CubeLight.BP_CubeLight_C"))
      (for _array_element_2 _outactors_2
        (if (== (Variables|/Game/Objects/Lights/BP_CubeLight.BP_CubeLight_C|GetGroup _array_element_2) (Variables|Default|GetGroup))
          (Default|ToggleonRandom _array_element_2)))
      (Timeline|Switch Reverse))))

(fn ConstructionScript
  (|CallParentFunction))