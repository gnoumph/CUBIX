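; BP_Text is a puzzle text actor whose characters light up while a BP_MagicCube is in its Box and the player's physics handle is active.
; The construction script fills the Char component from the Text variable.
; Overlap begin checks the handle and swaps Char's material, and Tick repeats the check while lit.
; Releasing the handle or any end overlap restores the default opaque material.
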(event OnComponentBeginOverlap(Box)
  (params (OverlappedComponent :type Primitive%20Component%20Object%20Reference) (OtherActor :type Actor%20Object%20Reference) (OtherComp :type Primitive%20Component%20Object%20Reference) (OtherBodyIndex :type Integer) (bFromSweep :type Boolean) (SweepResult :type Hit%20Result%20Structure%20%28by%20ref%29))
  (bind _char (Variables|Default|GetChar))
  (Utilities|Casting|CastToBP_MagicCube OtherActor)
  (bind _asbp_character (Utilities|Casting|CastToBP_Character (Game|GetPlayerCharacter 0)))
  (if (Variables|/Game/Blueprints/Datas/Character/BP_Character.BP_Character_C|GetPhysicsHandleActive _asbp_character)
    (Rendering|Material|SetMaterial _char 0 "/Game/Materials/MM_TextLight.MM_TextLight")
    (Variables|Default|SetOverlap? true)
    (else
      (Rendering|Material|SetMaterial _char 0 "/Engine/EngineMaterials/DefaultTextMaterialOpaque.DefaultTextMaterialOpaque")
      (Variables|Default|SetOverlap? false))))

(event OnComponentEndOverlap(Box)
  (params (OverlappedComponent :type Primitive%20Component%20Object%20Reference) (OtherActor :type Actor%20Object%20Reference) (OtherComp :type Primitive%20Component%20Object%20Reference) (OtherBodyIndex :type Integer))
  (Rendering|Material|SetMaterial (Variables|Default|GetChar) 0 "/Engine/EngineMaterials/DefaultTextMaterialOpaque.DefaultTextMaterialOpaque")
  (Variables|Default|SetOverlap? false))

(event EventTick
  (params (DeltaSeconds :type Float%20%28single-precision%29))
  (bind _char (Variables|Default|GetChar))
  (if (Variables|Default|GetOverlap?)
    (if (Variables|/Game/Blueprints/Datas/Character/BP_Character.BP_Character_C|GetPhysicsHandleActive (stale OnComponentBeginOverlap(Box) _asbp_character))
      (Rendering|Material|SetMaterial _char 0 "/Game/Materials/MM_TextLight.MM_TextLight")
      (Variables|Default|SetOverlap? true)
      (else
        (Rendering|Material|SetMaterial _char 0 "/Engine/EngineMaterials/DefaultTextMaterialOpaque.DefaultTextMaterialOpaque")
        (Variables|Default|SetOverlap? false)))))

(fn ConstructionScript
  (Rendering|Components|TextRender|SetText (Variables|Default|GetChar) (Variables|Default|GetText)))